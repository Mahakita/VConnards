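; Damageable component implementing D&D-style hit points, armor class, damage and healing.
; BeginPlay initializes HP, AC and per-type resistance, immunity and weakness arrays; attack rolls against AC trigger damage unless forced.
; Damage passes through Heavy Armor Master, flat reduction, type multipliers and a threshold, then drains temporary HP before current HP.
; Death, death-save handling and the approval prompt for temporary HP are stubs.
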(event Custom|TakeDamageEvent
  (params (Damage%20Amount :type Integer) (Damage%20Type :type Integer) (isAttack :type Boolean) (isHeavyArmorMaster :type Boolean))
  ;[1 0.1628 0.1131] Damage
  (bind _damagetaken (CallFunction|CalculateDamageReceived Damage%20Amount Damage%20Type isAttack isHeavyArmorMaster))
  (CallFunction|TakeorHealDamageFunc _damagetaken "NewEnumerator0" false)
  (|TriggerDeathSaves _damagetaken
    (:DeathSavesDone
      (if (and (== (Variables|HP|GetCurrent%20HP) 0) (not (Variables|HP|GetbIsAtZeroHP)))
        (Variables|HP|SetbIsAtZeroHP true)))))

(event Custom|Death
  ;[1 1 1] Death
)

(event Custom|Max%20HP%20Damage
  (params (Amount :type Integer))
  ;[1 0.1628 0.1131] Damage
  (CallFunction|TakeorHealDamageFunc Amount "NewEnumerator2" false))

(event Custom|AttackReceived
  (params (ForceHit :type Boolean) (Damage%20Amount :type Integer) (Damage%20Type :type Integer) (Roll%20Result :type Integer))
  ;[1 1 1] Attack Roll
  (if ForceHit
    (CallFunction|TakeDamageEvent 0 0 false false)
    (elif (>= Roll%20Result (Variables|AC|GetCurrent%20Armor%20Class))
      (CallFunction|TakeDamageEvent Damage%20Amount Damage%20Type true false)
      (else
        (Development|PrintString "Attack Missed")))))

(event Custom|Heal
  (params (Heal%20Amount :type Integer))
  ;[0.2285 1 0.287] Heal
  (CallFunction|TakeorHealDamageFunc Heal%20Amount "NewEnumerator1" false))

(event Custom|HasTakenDamage
  (params (DeathSavesFailed :type Integer))
  ;[1 1 1] Death Saves and Concentration checks
  (if (Variables|HP|GetbIsAtZeroHP)
    _))

(event Custom|TemporaryHPGain
  (params (Amount%20Gained :type Integer))
  ;[0.2486 0.4223 1] Temp HP
  (if (Variables|Default|GetApproval)
    (Variables|HP|SetTemporary%20HP Amount%20Gained)))

(event Custom|PromptUserForApproval
  ;[1 1 1] User Approval Prompt
)

(event Custom|Heal%20Max%20HP
  (params (Amount :type Integer))
  ;[0.2285 1 0.287] Heal
  (CallFunction|TakeorHealDamageFunc Amount "NewEnumerator3" false))

(event EventBeginPlay
  ;[1 1 1] Start
  (|SetHPs
    (:Done
      (|SetArmorClass)
      (|Setup_Res_Imm_Weak_Arrays))))

(fn MakeArrayfromStructDmgTypes
  (params (Struct_DamageTypes :type Struct%20Damage%20Types%20Structure%20%28by%20ref%29))
  (bind (_piercing _slashing _bludgeoning _fire _cold _lightning _thunder _poison _acid _necrotic _radiant _psychic _force _magicalpiercing _magicalslashing _magicalbludgeoning) (Utilities|Struct|BreakStruct_DamageTypes Struct_DamageTypes))
  (return (Utilities|Array|MakeArray _piercing _slashing _bludgeoning _fire _cold _lightning _thunder _poison _acid _necrotic _radiant _psychic _force _magicalpiercing _magicalslashing _magicalbludgeoning)))

(fn CalculateDamageReceived
  (params (DamageAmount :type Integer) (DamageType :type Integer) (isAttack :type Boolean) (hasHeavyArmorMasterFeat :type Boolean))
  (bind _modifieddamageamount (|HeavyArmorMaster hasHeavyArmorMasterFeat DamageType DamageAmount))
  (bind _modifieddamageamount_2 (|HomebrewDamageReduction _modifieddamageamount isAttack))
  (bind _returnvalue (|ModifyDmg_ResImmWeak _modifieddamageamount_2 DamageType))
  (bind _returnvalue_2 (Math|Float|Floor _returnvalue))
  (return (select (>= _returnvalue_2 (Variables|DamageModifiers|GetDamage%20Threshold)) _returnvalue_2 0)))

(fn TakeorHealDamageFunc
  (params (Amount :type Integer) (Type :type Enum_DamageInteractions%20Enum :default "NewEnumerator0") (AllowHigherThanMaxHP :type Boolean))
  (switch Utilities|FlowControl|Switch|SwitchonEnum_DamageInteractions Type
    (:NewEnumerator0
      ;[1 1 1] Damage Taken
      (if (> Amount (Variables|HP|GetTemporary%20HP))
        (Variables|HP|SetCurrent%20HP (Math|Integer|Max(Integer) (- (+ (Variables|HP|GetCurrent%20HP) (Variables|HP|GetTemporary%20HP)) Amount)))
        (Variables|HP|SetTemporary%20HP 0)
        (else
          (Variables|HP|SetTemporary%20HP (- (Variables|HP|GetTemporary%20HP) Amount))))
      (return))
    (:NewEnumerator1
      ;[1 1 1] Heals
      (Variables|HP|SetCurrent%20HP (Math|Integer|Min(Integer) (Variables|HP|GetCurrent%20Max%20HP) (+ (Variables|HP|GetCurrent%20HP) Amount))))
    (:NewEnumerator2
      ;[1 1 1] Max HP Dmg
      (Variables|HP|SetCurrent%20Max%20HP (Math|Integer|Max(Integer) (- (Variables|HP|GetCurrent%20Max%20HP) Amount))))
    (:NewEnumerator3
      ;[1 1 1] Max HP Heal / Increase
      (Variables|HP|SetCurrent%20Max%20HP (select AllowHigherThanMaxHP (+ (Variables|HP|GetCurrent%20Max%20HP) Amount) (Math|Integer|Min(Integer) (Variables|HP|GetMax%20HP) (+ (Variables|HP|GetCurrent%20Max%20HP) Amount)))))))