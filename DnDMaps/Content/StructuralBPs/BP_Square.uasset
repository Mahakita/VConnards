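; BP_Square is a grid tile actor whose look is set by its MaterialType.
; Its construction script picks the cube's material from MatInsts, then calls AlignToGrid, which labels the tile with rounded grid coordinates rather than moving it.
; One material type also adds a hay field mesh component using TopCenterOfCube, whose centred, random-yaw transform calculation is left unconnected.
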(event Custom|AlignToGrid
  (bind _self self)
  (bind _squaresize (Variables|Default|GetSquareSize))
  (bind _returnvalue (Transformation|GetActorLocation _self))
  (bind (_x _y) (Math|Vector|BreakVector _returnvalue))
  (Rendering|Components|TextRender|SetText (Variables|Default|GetY) (Utilities|Text|ToText(Integer) (Math|Float|Round (/ _y _squaresize))))
  (Rendering|Components|TextRender|SetText (Variables|Default|GetX) (Utilities|Text|ToText(Integer) (Math|Float|Round (/ _x _squaresize))))
  (switch int (Math|Conversions|ToInteger(Byte) (Variables|Default|GetMaterialType))
    (:1
      (|HayField))))

(event EventBeginPlay)

(event Collision|EventActorBeginOverlap
  (params (OtherActor :type Actor%20Object%20Reference)))

(fn ConstructionScript
  (Rendering|Material|SetMaterial (Variables|Default|GetCube1) 0 (Utilities|Array|Get(acopy) (Variables|Default|GetMatInsts) (Math|Conversions|ToInteger(Byte) (Variables|Default|GetMaterialType))))
  (CallFunction|AligntoGrid))