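; BP_PlayerCharacter is a player character Blueprint with an optional wings setting, configured in the Construction Script.
; With HasWings set, it moves StaticMesh10 to a relative height of half the upper Z bound of StaticMesh; otherwise it hides StaticMesh10.
; The event graph holds only disabled placeholder events, so this Blueprint adds no runtime logic there.
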(event EventBeginPlay
  (|CallParentFunction) ; This node is disabled and will not be called.\nDrag off pins to build functionality.
)

(event Collision|EventActorBeginOverlap
  (params (OtherActor :type Actor%20Object%20Reference))
  (|CallParentFunction OtherActor) ; This node is disabled and will not be called.\nDrag off pins to build functionality.
)

(event EventTick
  (params (DeltaSeconds :type Float%20%28single-precision%29))
  (|CallParentFunction DeltaSeconds) ; This node is disabled and will not be called.\nDrag off pins to build functionality.
)

(event Input|KeyboardEvents|W
  (params (Key :type Key%20Structure :default "None")))

(event Input|KeyboardEvents|A
  (params (Key :type Key%20Structure :default "None")))

(event Input|KeyboardEvents|S
  (params (Key :type Key%20Structure :default "None")))

(event Input|KeyboardEvents|D
  (params (Key :type Key%20Structure :default "None")))

(fn ConstructionScript
  (bind _staticmesh1_0 (Variables|Default|GetStaticMesh1_0))
  (|CallParentFunction)
  (if (Variables|Default|GetHasWings)
    (Transformation|SetRelativeLocation _staticmesh1_0 (Math|Vector|MakeVector 0.0 0.0 (/ (.Z (Math|Vector|BreakVector (.Max (Components|StaticMesh|GetLocalBounds (Variables|Default|GetStaticMesh))))) 2.0)) false false)
    (else
      (Rendering|SetVisibility _staticmesh1_0 false false))))