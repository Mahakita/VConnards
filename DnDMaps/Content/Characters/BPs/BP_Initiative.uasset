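; BP_Initiative steps through a Pawns array as an initiative order and relays movement commands to the currently selected pawn.
; InitiativeForward and InitiativeBackwards adjust InitiativeCounter, then SetPawn calls IsSelected on the previous and new pawns to toggle their selection arrows.
; Directional events forward unit-distance Move or Fly calls to CurrentPawn along fixed axes, with vertical movement only through Fly.
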(event Custom|InitiativeForward
  ;[1 1 1] InitiativeArrayManips
  (if (== (+ (Utilities|Array|Length (Variables|Default|GetPawns)) 1) (Variables|Default|GetInitiativeCounter))
    (Variables|Default|SetInitiativeCounter 0)
    (else
      (Math|Integer|IncrementInt (Variables|Default|GetInitiativeCounter)
        (:%20%20
          _))))
  (CallFunction|SetPawn))

(event Custom|M_FlyLeft
  ;[1 1 1] Pawn Movement
  (Default|Fly (Variables|Default|GetCurrentPawn) "0.000000,-1.000000,0.000000" 1))

(event Custom|M_FlyRight
  ;[1 1 1] Pawn Movement
  (Default|Fly (Variables|Default|GetCurrentPawn) "0.000000,1.000000,0.000000" 1))

(event Custom|M_FlyForwards
  ;[1 1 1] Pawn Movement
  (Default|Fly (Variables|Default|GetCurrentPawn) "1.000000, 0,0.000000" 1))

(event Custom|M_FlyBackwards
  ;[1 1 1] Pawn Movement
  (Default|Fly (Variables|Default|GetCurrentPawn) "-1.000000, 0,0.000000" 1))

(event Custom|InitiativeBackwards
  ;[1 1 1] InitiativeArrayManips
  (if (< (Variables|Default|GetInitiativeCounter) 0)
    (Variables|Default|SetInitiativeCounter (- (Utilities|Array|Length (Variables|Default|GetPawns)) 1))
    (else
      (Math|Integer|DecrementInt (Variables|Default|GetInitiativeCounter)
        (:%20%20
          _))))
  (CallFunction|SetPawn))

(event Custom|MUp
  ;[1 1 1] Pawn Movement
  (Default|Move (Variables|Default|GetCurrentPawn) "1.000000,0.000000, 0" 1))

(event Custom|MDown
  ;[1 1 1] Pawn Movement
  (Default|Move (Variables|Default|GetCurrentPawn) "-1.000000,0.000000, 0" 1))

(event Custom|MRight
  ;[1 1 1] Pawn Movement
  (Default|Move (Variables|Default|GetCurrentPawn) "0.000000,1.000000, 0" 1))

(event Custom|MLeft
  ;[1 1 1] Pawn Movement
  (Default|Move (Variables|Default|GetCurrentPawn) "0.000000,-1.000000, 0" 1))

(event Custom|SetPawn
  (bind _pawns (Variables|Default|GetPawns))
  (bind _initiativecounter (Variables|Default|GetInitiativeCounter))
  (bind _output (Utilities|Array|Get(acopy) _pawns _initiativecounter))
  ;[1 1 1] ToggleArrows
  (Utilities|IsValid (Variables|Default|GetPreviousPawn)
    (:Is%20Valid
      (Default|IsSelected (Variables|Default|GetPreviousPawn)))
    (:Is%20Not%20Valid
      _))
  (Utilities|IsValid _output
    (:Is%20Valid
      (bind _output_get (Variables|Default|SetCurrentPawn _output))
      (Default|IsSelected _output_get)
      (Variables|Default|SetPreviousPawn _output_get))))

(event Custom|M_FlyDown
  ;[1 1 1] Pawn Movement
  (Default|Fly (Variables|Default|GetCurrentPawn) "0, 0,-1.000000" 1))

(event Custom|M_FlyUp
  ;[1 1 1] Pawn Movement
  (Default|Fly (Variables|Default|GetCurrentPawn) "0, 0,1.000000" 1))

(event EventBeginPlay)

(event Collision|EventActorBeginOverlap
  (params (OtherActor :type Actor%20Object%20Reference)))

(event EventTick
  (params (DeltaSeconds :type Float%20%28single-precision%29)))

(fn ConstructionScript)