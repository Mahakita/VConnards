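; BP_Pawn is a grid-based character piece on a colored platform, with events to step, fly, go prone or stand up.
; Walk steps line-trace down at the neighboring square, ignoring foliage, and snap to the hit, while flying simply offsets by SquareMetrics.
; The construction script picks the platform mesh by Size, tints materials with PlatformColor, and places the sprite above the mesh bounds.
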(event Custom|Prone
  ;[1 1 1] Prone/StandUp
  (Transformation|SetRelativeTransform (Variables|Default|GetStaticMesh) (Variables|Preset|GetProneTransform) false false))

(event Custom|StandUp
  ;[1 1 1] Prone/StandUp
  (Transformation|SetRelativeTransform (Variables|Default|GetStaticMesh) (Variables|Preset|GetStandUpTransform) false false))

(event Custom|IsSelected
  (Rendering|ToggleVisibility (Variables|Default|GetArrowMesh) false))

(event Custom|MUp
  ;[1 1 1] MovementTriggerInEditor
  (CallFunction|Move "1.000000,0.000000, 0" 1))

(event Custom|MDown
  ;[1 1 1] MovementTriggerInEditor
  (CallFunction|Move "-1.000000,0.000000, 0" 1))

(event Custom|MRight
  ;[1 1 1] MovementTriggerInEditor
  (CallFunction|Move "0,1.000000, 0" 1))

(event Custom|MLeft
  ;[1 1 1] MovementTriggerInEditor
  (CallFunction|Move "0,-1.000000, 0" 1))

(event Custom|Fly
  (params (DirectionOfMove :type Vector) (Distance :type Integer))
  ;[1 1 1] FlyEvent
  (Transformation|AddActorWorldOffset (* (* DirectionOfMove (Variables|Default|GetSquareMetrics)) Distance)))

(event Custom|M_FlyRight
  ;[1 1 1] MovementTriggerInEditor
  (CallFunction|Fly "0,1.000000,0.000000" 1))

(event Custom|M_FlyLeft
  ;[1 1 1] MovementTriggerInEditor
  (CallFunction|Fly "0,-1.000000,0.000000" 1))

(event Custom|M_FlyUpwards
  ;[1 1 1] MovementTriggerInEditor
  (CallFunction|Fly "1.000000,0.000000,0.000000" 1))

(event Custom|M_FlyDownwards
  ;[1 1 1] MovementTriggerInEditor
  (CallFunction|Fly "-1.000000,0.000000,0.000000" 1))

(event Custom|Move
  (params (DirectionOfMove :type Vector) (Distance :type Integer))
  (bind _returnvalue (Transformation|GetActorLocation))
  (bind _squaremetrics (Variables|Default|GetSquareMetrics))
  (bind _returnvalue_2 (* DirectionOfMove _squaremetrics))
  (bind _returnvalue_3 (+ _returnvalue_2 _returnvalue))
  ;[1 1 1] WalkEvent
  (if (== Distance 1)
    (bind (_outhit _returnvalue_4) (Collision|LineTraceForObjects (+ _returnvalue_3 (Math|Vector|MakeVector 0.0 0.0 _squaremetrics) "5.000000,0.000000,81.000000") (- _returnvalue_3 "0, 0,157.000000") (Variables|Default|GetObjectsToHit) false (Variables|Default|GetFoliageInstances) "None"))
    (if _returnvalue_4
      (Transformation|SetActorLocation (.location _outhit) false true))))

(event Custom|M_Fly_Lower
  ;[1 1 1] MovementTriggerInEditor
  (CallFunction|Fly "0, 0,-1.000000" 1))

(event Custom|M_Fly_Higher
  ;[1 1 1] MovementTriggerInEditor
  (CallFunction|Fly "0, 0,1.000000" 1))

(event EventBeginPlay
  (bind _outactors (Actor|GetAllActorsOfClass "/Script/Foliage.InstancedFoliageActor"))
  (Variables|Default|SetFoliageInstances _outactors))

(fn ConstructionScript
  (|SetMeshColorOrSkipIfTextured
    (:then
      _)
    (:else
      _))
  (|PlatformStaticMeshSelection)
  (|PlatformDMIColorSet)
  (|SpriteSelection
    (:NewParam
      (|SetSpriteLocation)
      (Transformation|SetRelativeLocation (Variables|Default|GetScene) (* (.Max (Components|StaticMesh|GetLocalBounds (Variables|Default|GetStaticMesh))) "0, 0,1.000000") false true)
      (Rendering|SetVisibility (Variables|Default|GetArrowMesh) false false))))